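; LeverTrap_BP is a one-shot lever trap for killing Robot_AI enemies inside a configurable kill zone.
; On first interaction, a timeline swings the lever, then passes the trap to its referenced Telephone_wire through Initiate.
; LoopDamage, not called within this graph, deals heavy damage to every Robot_AI overlapping Killzone.
; The construction script places Killzone from the LeverTransform variable.
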(event EventInteractPass
  (Utilities|FlowControl|DoOnce false
    (:Completed
      (bind _newtrack_0 (Timeline|Timeline_0 Play)
        (:Update
          (Transformation|SetRelativeRotation (Variables|Default|GetLever) (Math|Rotator|Lerp(Rotator) "0, 0, 0" "0.000000, 0,115.000000" _newtrack_0 true) false false))
        (:Finished
          (bind _astelephone_wire (Utilities|Casting|CastToTelephone_wire (Variables|Default|GetTelephoneRef)))
          (Default|Initiate _astelephone_wire self))))))

(fn ConstructionScript
  (Transformation|SetRelativeTransform (Variables|Default|GetKillzone) (Variables|Default|GetLeverTransform) false false))

(fn LoopDamage
  (Development|PrintString "Kill Called")
  (bind _output_get (Variables|Default|SetEnemiestoapplydamage (Collision|GetOverlappingActors (Variables|Default|GetKillzone) "/Game/Masquerade_Proto/AI_Proto/AI_Basic/Robot_AI.Robot_AI_C" :!class /Script/Engine.PrimitiveComponent)))
  (for _array_element _output_get
    (Game|Damage|ApplyDamage _array_element 1e+03 0 0)
    (Development|PrintString "Kill")))