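; AnotherCamera is a prototype surveillance camera that rotates and watches for the player through PawnSensing.
; On BeginPlay a timeline lerps the actor's rotation from its starting orientation through a fixed negative yaw offset.
; When it sees a ProtoCharTFP pawn, it prints a debug message, stops the timeline to halt the rotation and sets its spotlight color to white.
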(event OnSeePawn(PawnSensing)
  (params (Pawn :type Pawn%20Object%20Reference))
  (Utilities|Casting|CastToProtoCharTFP Pawn
    (:then
      (Development|PrintString "SEEEN")
      (Utilities|FlowControl|Sequence
        (:then_0
          (bind _newtrack_1 (Timeline|Timeline_0 Stop)
            (:Update
              (Transformation|SetActorRotation (Math|Rotator|Lerp(Rotator) (Variables|Default|GetStartRot) (Variables|Default|GetEndRot) _newtrack_1)))))
        (:then_1
          (Rendering|Components|Light|SetLightColor (Variables|Default|GetSpotLight) "(R=1.000000,G=1.000000,B=1.000000,A=1.000000)" true))))
    (:CastFailed
      (Development|PrintString "failed"))))

(event EventBeginPlay
  (Variables|Default|SetStartRot (Transformation|GetActorRotation))
  (Variables|Default|SetEndRot (Math|Rotator|MakeRotator (.roll (Variables|Default|GetStartRot)) (.pitch (Variables|Default|GetStartRot)) (+ (.yaw (Variables|Default|GetStartRot)) -7e+01)))
  (bind _newtrack_1 (Timeline|Timeline_0 PlayFromStart)
    (:Update
      (Transformation|SetActorRotation (Math|Rotator|Lerp(Rotator) (Variables|Default|GetStartRot) (Variables|Default|GetEndRot) _newtrack_1)))))

(event Collision|EventActorBeginOverlap
  (params (OtherActor :type Actor%20Object%20Reference)))

(event EventTick
  (params (DeltaSeconds :type Float%20%28single-precision%29)))

(fn ConstructionScript)