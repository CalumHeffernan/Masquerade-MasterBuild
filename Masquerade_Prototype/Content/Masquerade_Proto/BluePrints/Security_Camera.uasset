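; Security camera prototype that patrols a detection sphere between waypoints and reacts to spotting the player.
; A timeline lerps the sphere to each of five billboard positions in a loop, pausing briefly between moves.
; When the player character overlaps the sphere, a visibility trace runs from the cube to the pawn.
; If nothing blocks the trace, the patrol stops and the spotlight turns red.
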(event OnComponentBeginOverlap(Sphere)
  (params (OverlappedComponent :type Primitive%20Component%20Object%20Reference) (OtherActor :type Actor%20Object%20Reference) (OtherComp :type Primitive%20Component%20Object%20Reference) (OtherBodyIndex :type Integer) (bFromSweep :type Boolean) (SweepResult :type Hit%20Result%20Structure%20%28by%20ref%29))
  ;[1 1 1] Can camera see the player?
  (if (== (Utilities|GetClass OtherActor) "/Game/Masquerade_Proto/PlayerChar/ProtoCharTFP.ProtoCharTFP_C")
    (bind (_outhit _returnvalue) (Collision|LineTraceByChannel (Transformation|GetWorldLocation (Variables|Default|GetCube)) (Transformation|GetActorLocation (Pawn|GetControlledPawn (Game|GetPlayerController 0))) "TraceTypeQuery1" false 0 "ForDuration"))
    (if _returnvalue
      (if (not (== (.HitItem (Collision|BreakHitResult _outhit)) 0))
        (Development|PrintString "nope"))
      (else
        (Utilities|FlowControl|Sequence
          (:then_0
            (Variables|Default|SetStopped? true)
            ;[1 1 1] waypoint attempt
            (bind _floattrack (Timeline|MoveTime Stop)
              (:Update
                (CallFunction|MoveCamera _floattrack))
              (:Finished
                (bind _result (Math|Integer|IncrementInt (Variables|Default|Getindexpos))
                  (:%20%20
                    (if (== _result (Utilities|Array|Length (Variables|Default|Getcamerapoint_array)))
                      (Variables|Default|Setindexpos 0))
                    (Variables|Default|Setstart%20location (Transformation|GetWorldLocation (Variables|Default|GetSphere)))
                    (Utilities|FlowControl|Delay 2.0)
                    (if (not (Variables|Default|GetStopped?))
                      (Timeline|MoveTime PlayFromStart)))))))
          (:then_1
            (Rendering|Components|Light|SetLightColor (Variables|Default|GetSpotLight) "(R=0.765625,G=0.011697,B=0.000000,A=1.000000)" true)))))))

(event EventBeginPlay
  ;[1 1 1] waypoint attempt
  (Variables|Default|Setcamerapoint_array (Utilities|Array|MakeArray (Variables|Default|GetBillboard) (Variables|Default|GetBillboard1) (Variables|Default|GetBillboard2) (Variables|Default|GetBillboard3) (Variables|Default|GetBillboard4)))
  (Variables|Default|Setindexpos 0)
  (Variables|Default|Setstart%20location (Transformation|GetWorldLocation (Variables|Default|GetSphere)))
  (bind _floattrack (Timeline|MoveTime PlayFromStart)
    (:Update
      (CallFunction|MoveCamera _floattrack))
    (:Finished
      (bind _result (Math|Integer|IncrementInt (Variables|Default|Getindexpos))
        (:%20%20
          (if (== _result (Utilities|Array|Length (Variables|Default|Getcamerapoint_array)))
            (Variables|Default|Setindexpos 0))
          (Variables|Default|Setstart%20location (Transformation|GetWorldLocation (Variables|Default|GetSphere)))
          (Utilities|FlowControl|Delay 2.0)
          (if (not (Variables|Default|GetStopped?))
            (Timeline|MoveTime PlayFromStart)))))))

(event Collision|EventActorBeginOverlap
  (params (OtherActor :type Actor%20Object%20Reference)))

(fn ConstructionScript)

(fn MoveCamera
  (params (Alpha :type Float%20%28single-precision%29))
  (Transformation|SetWorldLocation (Variables|Default|GetSphere) (Math|Vector|Lerp(Vector) (Variables|Default|Getstart%20location) (Transformation|GetWorldLocation (Utilities|Array|Get(acopy) (Variables|Default|Getcamerapoint_array) (Variables|Default|Getindexpos))) Alpha) false false))

(fn IsLoS?)