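; Destructible door actor that shatters when damaged and removes itself afterward.
; Any damage applies radius damage with impulse to the Destructible component at the actor's location.
; On fracture it adds a radial impulse at the hit point, disables collision and custom depth, then destroys itself after a short delay.
; Overlapping the Box turns on the Destructible's custom depth rendering; only fracture turns it off.
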(event OnComponentBeginOverlap(Box)
  (params (OverlappedComponent :type Primitive%20Component%20Object%20Reference) (OtherActor :type Actor%20Object%20Reference) (OtherComp :type Primitive%20Component%20Object%20Reference) (OtherBodyIndex :type Integer) (bFromSweep :type Boolean) (SweepResult :type Hit%20Result%20Structure%20%28by%20ref%29))
  (Rendering|SetRenderCustomDepth (Variables|Default|GetDestructible) true))

(event OnComponentFracture(Destructible)
  (params (HitPoint :type Vector%20%28by%20ref%29 :default "0, 0, 0") (HitDirection :type Vector%20%28by%20ref%29 :default "0, 0, 0"))
  (Physics|AddRadialImpulse (Variables|Default|GetDestructible) HitPoint 0.0 0.0 "RIF_Constant" false)
  (Collision|SetCollisionEnabled (Variables|Default|GetDestructible) "NoCollision")
  (Rendering|SetRenderCustomDepth (Variables|Default|GetDestructible) false)
  (Utilities|FlowControl|Delay 2.0)
  (Actor|DestroyActor))

(event EventBeginPlay)

(event Collision|EventActorBeginOverlap
  (params (OtherActor :type Actor%20Object%20Reference)))

(event EventTick
  (params (DeltaSeconds :type Float%20%28single-precision%29)))

(event Game|Damage|EventAnyDamage
  (params (Damage :type Float%20%28single-precision%29) (DamageType :type Damage%20Type%20Object%20Reference) (InstigatedBy :type Controller%20Object%20Reference) (DamageCauser :type Actor%20Object%20Reference))
  (Class|DestructibleComponent|ApplyRadiusDamage (Variables|Default|GetDestructible) 5e+01 (Transformation|GetActorLocation) 1e+02 2e+03 false))

(fn ConstructionScript)